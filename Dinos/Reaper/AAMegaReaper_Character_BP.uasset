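; Mega Reaper dino character Blueprint that adds a tap-or-hold aimed leap, adapted from Xenomorph jump logic.
; Jump input plays prep and launch montages while a clamped camera sphere trace sends the target to the server.
; An anim notify applies the calculated arc or look-based velocity, costs stamina and turns the body in flight; pressing again midair can brake it.
; A client timer drives rider crosshair and camera offset; attacks, dismounting and sleep cancel jumps.
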(event Custom|StartJumpIdle
  ;[0.4358 0 1] Start Throw Idle
  (Variables|Default|SetbPreventMovement true)
  (Variables|Local/DoNotEdit|SetbIsJumping true)
  (Class|PrimalCharacter|PlayAnimEx (Variables|Default|GetJumpPrepAnim) 1.0 "None" false false false false false 0.0 0.0))

(event Custom|ClearJump
  (params (ForceImmediateClear :type Boolean))
  ;[1 0.06229 0.1772] Clear throw
  (Variables|Default|SetbPreventMovement false)
  (Variables|Local/DoNotEdit|SetbIsJumping false)
  (Utilities|FlowControl|Sequence
    (:then_0
      (Variables|Local/DoNotEdit|SetUsingLaunchOffset false)
      (Variables|Local/DoNotEdit|SetJumpInstant true))
    (:then_1
      (Utilities|FlowControl|Delay 0.75)
      (if (not (Class|PrimalCharacter|IsMontagePlaying (Variables|Default|GetJumpPrepAnim) 0.0))
        _))))

(event Custom|Request%20Jump%20Response
  (params (isHoldingJump :type Boolean))
  ;[0 0.05982 1] Jump Response
  (if isHoldingJump
    (if (Utilities|Enum|Equal(Enum) (Variables|/Script/Engine.CharacterMovementComponent|GetMovementMode (Variables|Character|GetCharacterMovement)) "MOVE_Falling")
      (CallFunction|ServerArrestMovement)
      (elif (not (Variables|Local/DoNotEdit|GetbIsJumping))
        (Utilities|AllowOncePerTime 0.8)
        (CallFunction|ProcessJump)))
    (elif (Variables|Local/DoNotEdit|GetbIsJumping)
      (Utilities|AllowOncePerTime 0.8)
      (CallFunction|ProcessLaunch))))

(event Custom|Multi_TraceTargetDir
  (params (AimLoc :type Vector) (AimHit :type Boolean))
  ;[0.1086 0.03835 0.43] Set Server trace infos
  (Variables|Local/DoNotEdit|SetJumpTraceLoc AimLoc)
  (Variables|Local/DoNotEdit|SetJumpTraceHit AimHit))

(event Custom|AnimNotify_JumpStart
  (if (Networking|IsServer)
    (Utilities|FlowControl|Sequence
      (:then_0
        ;[1 0.101 0] Launch characters
        (CallFunction|LaunchatTracePoint)
        (CallFunction|DelayedClearJumping))
      (:then_1
        ;[0.2572 1 0.05745] Stamina Cost
        (if (Networking|IsServer)
          (Class|PrimalCharacterStatusComponent|ModifyCurrentStatusValue (Variables|Default|GetMyCharacterStatusComponent) "Stamina" (* (Variables|Default|GetJumpLaunchStaminaCost) -1.0) false false false false 0 false false))))))

(event Custom|Multi_SetPreventMovement
  (params (NewPreventMovement :type Boolean))
  ;[1 0.6727 0] Set Prevent Movement
  (Variables|Default|SetbPreventMovement NewPreventMovement))

(event Custom|UpdateAllJumpRotation
  ;[0.2599 0.9905 1] Update prevent turn
  (CallFunction|UpdateJumpRotation))

(event Custom|UpdateJumpRotation
  (bind _returnvalue (Transformation|GetActorRotation))
  (bind _yaw (Class|KismetMathLibrary|BreakRot _returnvalue))
  ;[0.2599 0.9905 1] Update prevent turn
  (bind _return_value (CallFunction|ShouldStopJumpRotation))
  (if (not _return_value)
    (Transformation|SetActorRotation (Math|Rotator|MakeRotator 0.0 (+ _yaw (Math|Interpolation|FInterptoConstant 0.0 (CallFunction|ShortestAngleDistance _yaw (.Yaw (Class|KismetMathLibrary|BreakRot (Math|Rotator|MakeRotfromX (Variables|Default|GetJumpRotationTargetDir))))) (Utilities|Time|GetWorldDeltaSeconds) 55.0)) 0.0))
    (Class|KismetSystemLibrary|SetTimerforNextTick self "UpdateJumpRotation" false)))

(event Custom|Server_TraceTargetDir
  (params (AimLoc :type Vector) (AimHit :type Boolean) (JumpInstant :type Boolean))
  ;[0.1086 0.03835 0.43] Set Server trace infos
  (Variables|Local/DoNotEdit|SetJumpTraceLoc AimLoc)
  (Variables|Local/DoNotEdit|SetJumpTraceHit AimHit)
  (Variables|Local/DoNotEdit|SetJumpInstant JumpInstant)
  (CallFunction|MultiTraceTargetDir AimLoc AimHit))

(event Custom|DelayedClearJumping
  ;[1 0 0.1109] Delayed Launch
  (Variables|Local/DoNotEdit|SetbIsJumping false)
  (Utilities|FlowControl|Delay 1.0)
  (CallFunction|ClearJump false))

(event Custom|DelayedPress
  ;[0.3488 1 0.9618] Space/A button inputs
  (Variables|Local/DoNotEdit|SetJumpInstant false)
  (CallFunction|JumpTrace)
  (CallFunction|RequestJumpResponse true))

(event Custom|ServerArrestMovement
  (bind _returnvalue (Class|Actor|GetWorld))
  (bind _jumplaunchtime (Variables|Default|GetJumpLaunchTime))
  (bind _returnvalue_2 (Class|VictoryCore|TimeSince _returnvalue _jumplaunchtime))
  ;[1 1 1] Arrest Movement
  (if (Math|Boolean|ANDBoolean (Networking|IsServer) (Utilities|Enum|Equal(Enum) (Variables|/Script/Engine.CharacterMovementComponent|GetMovementMode (Variables|Character|GetCharacterMovement)) "MOVE_Falling") (>= _returnvalue_2 0.25) (<= _returnvalue_2 (Variables|Default|GetTimeToAllowArrestMovement)) (Variables|Default|GetbAllowArrestMovement))
    (Utilities|FlowControl|DoOnce false
      (:Completed
        (Class|PrimalCharacter|BPNetSetCharacterMovementVelocity true (|CalcSlowedVelocity_2 (Variables|/Script/Engine.MovementComponent|GetVelocity (Variables|Character|GetCharacterMovement))) false "MOVE_None")
        (Variables|Default|SetbAllowArrestMovement false)))))

(event Custom|ResetArrestMovement
  ;[1 1 1] Arrest Movement
  (Variables|Default|SetbAllowArrestMovement false)
  (Utilities|FlowControl|DoOnce false) ; enters at Reset
)

(event EventOnJumpPressed
  ;[0.3488 1 0.9618] Space/A button inputs
  (Utilities|Time|SetTimerbyFunctionName self "DelayedPress" (Variables|Default|GetJumpHoldTimeAllowance))
  (CallFunction|JumpTrace)
  (CallFunction|RequestJumpResponse true))

(event EventOnJumpReleased
  ;[0.3488 1 0.9618] Space/A button inputs
  (if (Class|KismetSystemLibrary|IsTimerActive self "DelayedPress")
    (Utilities|Time|ClearTimerbyFunctionName self "DelayedPress")
    (Variables|Local/DoNotEdit|SetJumpInstant true))
  (CallFunction|JumpTrace)
  (CallFunction|RequestJumpResponse false))

(event EventOnSetDeath
  ;[1 1 1] Remove PS on death
  (|CallParentFunction)
  (Utilities|FlowControl|Delay 0.2)
  (Components|Activation|Deactivate (Variables|Default|GetAlphaPS)))

(fn ConstructionScript
  (|CallParentFunction))

(fn GetClampedLookDir
  (params (LimitLowerPitch :type Boolean))
  (bind _returnvalue (Transformation|GetActorForwardVector))
  (bind _returnvalue_2 (Pawn|GetControlRotation :!class /Script/Engine.Pawn))
  (bind _xenojumpaimlimit (Variables|Default|GetXenoJumpAimLimit))
  (bind (_pitch _yaw) (Class|KismetMathLibrary|BreakRot _returnvalue_2))
  (bind _returnvalue_3 (Math|Rotator|MakeRotfromX _returnvalue))
  (bind _returnvalue_4 (* _xenojumpaimlimit -1.0))
  (bind _yaw_2 (Class|KismetMathLibrary|BreakRot _returnvalue_3))
  (bind _difference (CallFunction|ShortestAngleDistance _yaw_2 _yaw))
  (bind _returnvalue_5 (Math|Float|Clamp(Float) _difference _returnvalue_4 _xenojumpaimlimit))
  (bind _returnvalue_6 (+ _yaw_2 _returnvalue_5))
  (return (Math|Vector|GetForwardVector (Class|KismetMathLibrary|MakeRot (Math|Float|SelectFloat 45.0 (Math|Float|Clamp(Float) _pitch (Math|Float|SelectFloat 15.0 -9e+01 LimitLowerPitch) 9e+01) LimitLowerPitch) (+ _returnvalue_6 (Math|Float|SelectFloat 3.6e+02 0.0 (<= _returnvalue_6 -1.8e+02)) (Math|Float|SelectFloat -3.6e+02 0.0 (> _returnvalue_6 1.8e+02))) 0.0))))

(fn ShortestAngleDistance
  (params (AngleCurrent :type Float%20%28single-precision%29) (AngleTarget :type Float%20%28single-precision%29))
  (bind _returnvalue (- AngleTarget AngleCurrent))
  (return (+ _returnvalue (Math|Float|SelectFloat 3.6e+02 0.0 (<= _returnvalue -1.8e+02)) (Math|Float|SelectFloat -3.6e+02 0.0 (> _returnvalue 1.8e+02)))))

(fn ShouldStopJumpRotation
  (bind _jumplaunchtime (Variables|Default|GetJumpLaunchTime))
  (LocalVariables|SetShouldStop false)
  (Utilities|FlowControl|Sequence
    (:then_0
      (bind _asshootergamestate (Utilities|Casting|CastToShooterGameState (Game|GetGameState)))
      (bind _returnvalue (Class|ShooterGameState|GetNetworkTimeDelta _asshootergamestate _jumplaunchtime false))
      (LocalVariables|SetShouldStop (Math|Boolean|ORBoolean (> (Math|Conversions|ToFloat(Integer) _returnvalue) 5.0) (== _jumplaunchtime 0.0) (Math|Float|NearlyEqual(Float) (.Yaw (Class|KismetMathLibrary|BreakRot (Transformation|GetActorRotation))) (.Yaw (Class|KismetMathLibrary|BreakRot (Math|Rotator|MakeRotfromX (Variables|Default|GetJumpRotationTargetDir)))) 0.0001) (not (Utilities|Enum|Equal(Enum) (Variables|/Script/Engine.CharacterMovementComponent|GetMovementMode (Variables|Character|GetCharacterMovement)) "MOVE_Falling")) (Math|Float|NearlyEqual(Float) (Math|Vector|VectorLength (Variables|/Script/Engine.MovementComponent|GetVelocity (Variables|Character|GetCharacterMovement))) 0.0 5.0))))
    (:then_1
      (return (LocalVariables|GetShouldStop)))))

(fn JumpTrace
  (bind _returnvalue (CallFunction|GetClampedLookDir false))
  (if (Variables|Local/DoNotEdit|GetbIsJumping)
    (Utilities|FlowControl|Sequence
      (:then_0
        (bind _asplayercontroller (Utilities|Casting|CastToPlayerController (Pawn|GetController)))
        (bind (_outhit _returnvalue_2) (Class|KismetSystemLibrary|SphereTraceSingleNEW (+ (Camera|GetCameraLocation (Variables|/Script/Engine.PlayerController|GetPlayerCameraManager _asplayercontroller)) (* _returnvalue 1e+02)) (+ (Camera|GetCameraLocation (Variables|/Script/Engine.PlayerController|GetPlayerCameraManager _asplayercontroller)) (* _returnvalue (* (Variables|Default|GetJumpForceMult) (Variables|Default|GetTraceLength)))) 5e+01 "TraceTypeQuery9" false 0 "None" true))
        (Variables|Local/DoNotEdit|SetJumpTraceHit _returnvalue_2)
        (if _returnvalue_2
          (Variables|Local/DoNotEdit|SetJumpTraceLoc (+ (.ImpactPoint (Collision|BreakHitResult _outhit)) (Math|Vector|MakeVector 0.0 0.0 (+ (Math|Float|Clamp(Float) (* (/ (Math|Vector2D|Vector2DLength (Math|Vector2D|MakeVector2D (.X (Math|Vector|BreakVector (- (.ImpactPoint (Collision|BreakHitResult _outhit)) (+ (Transformation|GetActorLocation) "0, 0,200.000000")))) (.Y (Math|Vector|BreakVector (- (.ImpactPoint (Collision|BreakHitResult _outhit)) (+ (Transformation|GetActorLocation) "0, 0,200.000000")))))) 2e+03) 5.5) 25.0 1.5e+02) (Math|Float|Lerp 175.0 275.0 (Math|Float|Clamp(Float) (/ (.Z (Math|Vector|BreakVector (- (.ImpactPoint (Collision|BreakHitResult _outhit)) (+ (Transformation|GetActorLocation) "0, 0,200.000000")))) 1e+03)))))))
          (else
            (Variables|Local/DoNotEdit|SetJumpTraceLoc "0, 0, 0"))))
      (:then_1
        (CallFunction|ServerTraceTargetDir (Variables|Local/DoNotEdit|GetJumpTraceLoc) (Variables|Local/DoNotEdit|GetJumpTraceHit) (Variables|Local/DoNotEdit|GetJumpInstant))))))

(fn ProcessJump
  (Utilities|FlowControl|Sequence
    (:then_0
      (if (Utilities|Enum|Equal(Enum) (Variables|/Script/Engine.CharacterMovementComponent|GetMovementMode (Variables|Character|GetCharacterMovement)) "MOVE_Walking")
        (bind _returnvalue (Class|PrimalDinoCharacter|CanAttack 5))
        (if (and _returnvalue (not (Class|PrimalCharacter|IsinStatusState "Encumbered")))
          (CallFunction|StartJumpIdle))))))

(fn ProcessLaunch
  (Utilities|FlowControl|Sequence
    (:then_0
      (if (Utilities|Enum|Equal(Enum) (Variables|/Script/Engine.CharacterMovementComponent|GetMovementMode (Variables|Character|GetCharacterMovement)) "MOVE_Walking")
        (CallFunction|MultiSetPreventMovement false)
        (Class|PrimalCharacter|PlayAnimEx (Variables|Default|GetJumpStartAnim) 1.0 "None" true true false false false 0.0 0.0)
        (CallFunction|MultiTraceTargetDir (Variables|Local/DoNotEdit|GetJumpTraceLoc) (Variables|Local/DoNotEdit|GetJumpTraceHit))))))

(fn LaunchatTracePoint
  (bind _self self)
  (bind _returnvalue (CallFunction|GetLaunchDirection _self))
  (Class|PrimalCharacter|BPNetSetCharacterMovementVelocity _self true _returnvalue true "MOVE_Falling")
  (Variables|Default|SetJumpLaunchTime (Utilities|Time|GetGameTimeinSeconds) true)
  (Variables|Default|SetJumpRotationTargetDir _returnvalue true)
  (Class|KismetSystemLibrary|SetTimerforNextTick self "UpdateAllJumpRotation" false)
  (Variables|Default|SetbAllowArrestMovement true))

(fn GetLaunchDirection
  (params (CalcActor :type Actor%20Object%20Reference))
  (bind _returnvalue (Transformation|GetActorLocation CalcActor))
  (bind _jumpinstant (Variables|Local/DoNotEdit|GetJumpInstant))
  (bind _jumpfwdstrengthmax (Variables|Default|GetJumpFwdStrengthMax))
  (bind _jumphorizontaldistancemin (Variables|Default|GetJumpHorizontalDistanceMin))
  (bind _jumpverticaldistancemin (Variables|Default|GetJumpVerticalDistanceMin))
  (bind _jumptraceloc (Variables|Local/DoNotEdit|GetJumpTraceLoc))
  (bind _launchedcharactersapextraveltime (Variables|Default|GetLaunchedCharactersApexTravelTime))
  (bind _jumpforcemult (Variables|Default|GetJumpForceMult))
  (bind _returnvalue_2 (/ _launchedcharactersapextraveltime 4.0))
  (bind _returnvalue_3 (- _jumptraceloc _returnvalue))
  (bind _returnvalue_4 (* _jumpfwdstrengthmax _jumpforcemult))
  (bind (_x _y) (Math|Vector|BreakVector _returnvalue_3))
  (bind (_x_2 _y_2 _z) (Math|Vector|BreakVector _returnvalue_3))
  (bind _returnvalue_5 (* 8e+03 _returnvalue_2))
  (bind _returnvalue_6 (Math|Vector2D|MakeVector2D _x_2 _y_2))
  (bind _returnvalue_7 (Math|Float|Absolute(Float) _z))
  (bind _returnvalue_8 (Math|Vector2D|Vector2DLength _returnvalue_6))
  (bind _returnvalue_9 (<= _returnvalue_7 _jumpverticaldistancemin))
  (bind _returnvalue_10 (/ _returnvalue_8 _returnvalue_5))
  (bind _returnvalue_11 (< _returnvalue_8 _jumphorizontaldistancemin))
  (bind _returnvalue_12 (and _returnvalue_11 _returnvalue_9))
  (bind _returnvalue_13 (Math|Float|Min(Float) _returnvalue_10 1.0))
  (bind _returnvalue_14 (* _returnvalue_13 9e+01))
  (bind _returnvalue_15 (Math|Trig|Sin(Degrees) _returnvalue_14))
  (bind _returnvalue_16 (Math|Float|Lerp 0.0001 _returnvalue_4 _returnvalue_15))
  (bind _returnvalue_17 (/ _returnvalue_16 2.0))
  (return (* (Math|Vector|SelectVector (+ (* (Math|Vector|Normalize (Math|Vector|MakeVector _x _y 0.0)) _returnvalue_17) (* (Transformation|GetActorUpVector) (Math|Float|Clamp(Float) (+ (* (/ _returnvalue_8 _returnvalue_16) (* (Variables|/Script/Engine.CharacterMovementComponent|GetGravityScale (Variables|Character|GetCharacterMovement)) (Math|Float|MakeLiteralFloat 9.8e+02))) (/ _z (/ _returnvalue_8 _returnvalue_17))) (Variables|Default|GetJumpUpStrengthMin) (* (Variables|Default|GetJumpUpStrengthMax) (Variables|Default|GetJumpForceMult))))) (* (|NoTraceLookVelocity_2_2) (Variables|Default|GetJumpForceMult)) (Math|Boolean|ANDBoolean (Variables|Local/DoNotEdit|GetJumpTraceHit) (not _jumpinstant) (not _returnvalue_12))) (Math|Float|SelectFloat 0.4 (Math|Float|SelectFloat 0.6 1.0 _jumpinstant) _returnvalue_12))))

(fn BPDoAttack
  (params (AttackIndex :type Integer))
  (|CallParentFunction AttackIndex)
  (CallFunction|ServerStopJump))

(fn ServerStopJump
  (bind _jumpprepanim (Variables|Default|GetJumpPrepAnim))
  (CallFunction|ClearJump true)
  (CallFunction|ResetArrestMovement)
  (if (Class|PrimalCharacter|IsMontagePlaying _jumpprepanim 0.0)
    (Class|PrimalCharacter|StopAnimEx _jumpprepanim true true 0.0)))

(fn BPNotifyClearRider
  (params (RiderClearing :type Shooter%20Character%20Object%20Reference))
  (|CallParentFunction RiderClearing)
  (CallFunction|ServerStopJump))

(fn BPonMovementModeChangedNotify
  (params (PrevMovementMode :type EMovementMode%20Enum :default "MOVE_None") (PreviousCustomMode :type Byte :default 0))
  (bind _charactermovement (Variables|Character|GetCharacterMovement))
  (bind _movementmode (Variables|/Script/Engine.CharacterMovementComponent|GetMovementMode _charactermovement))
  (|CallParentFunction "MOVE_None" 0)
  (Utilities|FlowControl|Sequence
    (:then_0
      (if (not (Utilities|Enum|Equal(Enum) (Variables|/Script/Engine.CharacterMovementComponent|GetMovementMode (Variables|Character|GetCharacterMovement)) "MOVE_Walking"))
        (CallFunction|ServerStopJump)))
    (:then_1
      (if (or (Utilities|Enum|Equal(Enum) _movementmode "MOVE_Walking") (Utilities|Enum|Equal(Enum) _movementmode "MOVE_Falling"))
        (CallFunction|UpdateJumpRotation)))))

(fn BPCharacterSleeped
  (|CallParentFunction)
  (CallFunction|ServerStopJump))

(fn BPTimerNonDedicated
  (bind _returnvalue (Transformation|GetActorForwardVector))
  (bind _returnvalue_2 (Transformation|GetActorLocation))
  (bind _returnvalue_3 (Pawn|GetControlRotation :!class /Script/Engine.Pawn))
  (bind _xenojumpaimlimit (Variables|Default|GetXenoJumpAimLimit))
  (bind _jumpprepanim (Variables|Default|GetJumpPrepAnim))
  (bind _jumptraceloc (Variables|Local/DoNotEdit|GetJumpTraceLoc))
  (bind _returnvalue_4 (- _jumptraceloc _returnvalue_2))
  (bind _returnvalue_5 (Class|PrimalCharacter|IsMontagePlaying _jumpprepanim 0.0))
  (bind (_pitch _yaw) (Class|KismetMathLibrary|BreakRot _returnvalue_3))
  (bind _returnvalue_6 (Math|Rotator|MakeRotfromX _returnvalue))
  (bind _returnvalue_7 (== _xenojumpaimlimit 0.0))
  (bind (_x _y _z) (Math|Vector|BreakVector _returnvalue_4))
  (bind _yaw_2 (Class|KismetMathLibrary|BreakRot _returnvalue_6))
  (bind _returnvalue_8 (<= _pitch 9e+01))
  (bind _returnvalue_9 (Math|Rotator|Delta(Rotator) (Math|Rotator|MakeRotator 0.0 _yaw_2 0.0) (Math|Rotator|MakeRotator 0.0 _yaw 0.0)))
  (bind _yaw_3 (Class|KismetMathLibrary|BreakRot _returnvalue_9))
  (bind _returnvalue_10 (Math|Float|Absolute(Float) _yaw_3))
  (bind _returnvalue_11 (<= _returnvalue_10 _xenojumpaimlimit))
  (bind _returnvalue_12 (and _returnvalue_11 _returnvalue_8))
  (bind _returnvalue_13 (or _returnvalue_12 _returnvalue_7))
  (|CallParentFunction)
  (if (and (Class|PrimalDinoCharacter|BPIsTamed) (Variables|Default|GetbHasRider))
    (if (Variables|Local/DoNotEdit|GetbIsJumping)
      (CallFunction|JumpTrace)
      (Variables|Default|SetbForceRiderDrawCrosshair (Math|Boolean|ANDBoolean (Variables|Local/DoNotEdit|GetJumpTraceHit) (not (and (< (Math|Vector2D|Vector2DLength (Math|Vector2D|MakeVector2D _x _y)) (Variables|Default|GetJumpHorizontalDistanceMin)) (<= (Math|Float|Absolute(Float) _z) (Variables|Default|GetJumpVerticalDistanceMin)))) (and _returnvalue_13 _returnvalue_5)))
      (else
        (Variables|Default|SetbForceRiderDrawCrosshair _returnvalue_13)))
    (if _returnvalue_5
      (Variables|Default|SetTPVCameraOffsetMultiplier (Math|Interpolation|VInterptoConstant (Variables|Default|GetTPVCameraOffsetMultiplier) "-9.000000,1.000000,1.050000" (Utilities|Time|GetWorldDeltaSeconds) 3.0))
      (Variables|Local/DoNotEdit|SetUsingLaunchOffset true)
      (elif (or (Variables|Local/DoNotEdit|GetUsingLaunchOffset) (Utilities|Enum|Equal(Enum) (Variables|/Script/Engine.CharacterMovementComponent|GetMovementMode (Variables|Character|GetCharacterMovement)) "MOVE_Falling"))
        (Variables|Default|SetTPVCameraOffsetMultiplier (Math|Interpolation|VInterptoConstant (Variables|Default|GetTPVCameraOffsetMultiplier) "-10.000000,1.000000,0.750000" (Utilities|Time|GetWorldDeltaSeconds) 3.0))
        (else
          (bind _returnvalue_14 (Class|VictoryCore|GetDefaultObject self))
          (bind _asprimaldinocharacter (Utilities|Casting|CastToPrimalDinoCharacter _returnvalue_14))
          (Variables|Default|SetTPVCameraOffsetMultiplier (Math|Interpolation|VInterptoConstant (Variables|Default|GetTPVCameraOffsetMultiplier) (Variables|/Script/ShooterGame.PrimalCharacter|GetTPVCameraOffsetMultiplier _asprimaldinocharacter) (Utilities|Time|GetWorldDeltaSeconds) 1.0)))))))

(fn BPNotifySetRider
  (params (RiderSetting :type Shooter%20Character%20Object%20Reference))
  (|CallParentFunction RiderSetting)
  (Variables|Default|SetBPTimerNonDedicatedMax 0.01)
  (Variables|Default|SetBPTimerNonDedicatedMin 0.01))