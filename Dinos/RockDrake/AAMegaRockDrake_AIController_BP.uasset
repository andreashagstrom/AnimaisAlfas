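; AI controller for the Mega Rock Drake that manages the camouflage of wild, untamed drakes.
; When its target changes, it runs the parent logic and casts the controlled pawn to the Rock Drake character.
; If the drake is untamed and no valid target remains, it sets camo to the drake's wild camo preference and prints a "LOST TARGET" debug string.
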(fn ConstructionScript
  (|CallParentFunction))

(fn BPNotifyTargetSet
  (|CallParentFunction)
  (bind _asrockdrake_character_bp_c (Utilities|Casting|CastToRockDrake_Character_BP (Pawn|GetControlledPawn)))
  (if (not (Class|PrimalDinoCharacter|BPIsTamed _asrockdrake_character_bp_c))
    (Utilities|IsValid (Variables|Default|GetTarget)
      (:Is%20Not%20Valid
        (Default|NetSetUseCamo _asrockdrake_character_bp_c (Variables|/Game/Aberration/Dinos/RockDrake/RockDrake_Character_BP.RockDrake_Character_BP_C|GetbWildDrakeWantsToCamo _asrockdrake_character_bp_c))
        (Development|PrintString "LOST TARGET" true true "(R=1.000000,G=0.037960,B=0.000000,A=1.000000)")))))